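; Enemy AI character that wanders to random reachable points, chases the player when seen, and stages a catch.
; Tick issues delayed roaming moves while not chasing; PawnSensing starts AIMoveTo on the player, with a retriggerable delay clearing the chase after sight is lost.
; CatchPlayer runs a short self-calling delay loop that turns the player toward the enemy, plays a montage, then resets.
; Startbrr and Stopbrr switch between sprint and walk speeds.
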(event OnSeePawn(PawnSensing)
  (params (Pawn :type Pawn%20Object%20Reference))
  (bind _asfpsmovement (Utilities|Casting|CastToFPSmovement Pawn))
  (if (not (Variables|Default|GetCaught?))
    (Utilities|FlowControl|Sequence
      (:then_0
        (Variables|Default|SetCan%20See%20Player? true)
        (Variables|Default|SetIsChasing? true)
        (AI|AIMoveTo self "0, 0, 0" _asfpsmovement 5.0 false
          (:then
            (Utilities|FlowControl|DoOnce false))))
      (:then_1
        (Utilities|FlowControl|RetriggerableDelay 0.6)
        (Variables|Default|SetCan%20See%20Player? false)
        (Variables|Default|SetIsChasing? false)))))

(event Custom|Catch%20Player
  (bind _returnvalue (Game|GetPlayerController 0))
  (Variables|Default|SetCaught? true)
  (Variables|Default|SetShould%20Loop? true)
  (bind _asfpsmovement (Utilities|Casting|CastToFPSmovement (Game|GetPlayerCharacter 0)))
  (if (Variables|Default|GetShould%20Loop?)
    (Utilities|FlowControl|Delay 0.001)
    (Transformation|SetActorRotation _asfpsmovement (Math|Rotator|FindLookatRotation (Transformation|GetActorLocation _asfpsmovement) (Transformation|GetActorLocation)))
    (Pawn|SetControlRotation _returnvalue (Math|Interpolation|RInterpTo (Pawn|GetControlRotation _returnvalue :!class /Script/Engine.Controller) (Math|Rotator|FindLookatRotation (Transformation|GetActorLocation _asfpsmovement) (Transformation|GetActorLocation)) 0.0 0.0))
    (CallFunction|RotationLoop)
    (Utilities|FlowControl|DoOnce false :!label _label
      (:Completed
        (Utilities|FlowControl|Sequence
          (:then_0
            (Animation|PlayAnimMontage 0 1.0 "None")
            (Utilities|FlowControl|Delay 1.0)
            (Variables|Default|SetCaught? false))
          (:then_1
            (Utilities|FlowControl|Delay 0.5)
            (Variables|Default|SetShould%20Loop? false)
            (goto _label Reset)))))))

(event Custom|Rotation%20Loop
  (bind _returnvalue (Game|GetPlayerController 0))
  (if (Variables|Default|GetShould%20Loop?)
    (Utilities|FlowControl|Delay 0.001)
    (Transformation|SetActorRotation (stale Custom|Catch%20Player _asfpsmovement) (Math|Rotator|FindLookatRotation (Transformation|GetActorLocation (stale Custom|Catch%20Player _asfpsmovement)) (Transformation|GetActorLocation)))
    (Pawn|SetControlRotation _returnvalue (Math|Interpolation|RInterpTo (Pawn|GetControlRotation _returnvalue :!class /Script/Engine.Controller) (Math|Rotator|FindLookatRotation (Transformation|GetActorLocation (stale Custom|Catch%20Player _asfpsmovement)) (Transformation|GetActorLocation)) 0.0 0.0))
    (CallFunction|RotationLoop)
    (Utilities|FlowControl|DoOnce false :!label _label
      (:Completed
        (Utilities|FlowControl|Sequence
          (:then_0
            (Animation|PlayAnimMontage 0 1.0 "None")
            (Utilities|FlowControl|Delay 1.0)
            (Variables|Default|SetCaught? false))
          (:then_1
            (Utilities|FlowControl|Delay 0.5)
            (Variables|Default|SetShould%20Loop? false)
            (goto _label Reset)))))))

(event EventTick
  (params (DeltaSeconds :type Float%20%28single-precision%29))
  (if (not (Variables|Default|GetIsChasing?))
    (Utilities|FlowControl|Delay (Math|Random|RandomFloatinRange 2.0 5.0))
    (AI|AIMoveTo self (.RandomLocation (AI|Navigation|GetRandomReachablePointinRadius (Transformation|GetActorLocation) 1.5e+03 0 0)) 0 5.0 false)))

(fn ConstructionScript)

(fn Startbrr
  (Variables|/Script/Engine.CharacterMovementComponent|SetMaxWalkSpeed (Variables|Character|GetCharacterMovement) (Variables|Default|GetSprint)))

(fn Stopbrr
  (Variables|/Script/Engine.CharacterMovementComponent|SetMaxWalkSpeed (Variables|Character|GetCharacterMovement) (Variables|Default|GetWalking)))