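; First-person player character Blueprint handling look, movement, sprinting and a flashlight that can be picked up.
; Movement follows control yaw, and both movement axes feed shared logic that starts a running or walking camera shake on every axis event, with walking shake scaled by input.
; Sprint switches max walk speed and the shake choice.
; The pickupflashlite event reveals the flashlight mesh and lets F toggle its spotlight.
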(event Custom|pickupflashlite
  (Rendering|SetVisibility (Variables|Default|Getflashlite) true false)
  (Variables|Default|Setpickeduptorch true))

(event Input|ActionEvents|InputActionSprint
  (params (Key :type Key%20Structure :default "None"))
  (:Pressed
    (CallFunction|Startbrr)
    (Variables|Default|Setrunningshake true))
  (:Released
    (CallFunction|Stopbrr)
    (Variables|Default|Setrunningshake false)))

(event Input|AxisEvents|InputAxisForward/Backward
  (params (AxisValue :type Float%20%28single-precision%29))
  (bind _returnvalue (Game|GetPlayerController 0))
  (Pawn|Input|AddMovementInput (Math|Vector|GetForwardVector (Math|Rotator|MakeRotator 0.0 0.0 (.Yaw (Math|Rotator|BreakRotator (Pawn|GetControlRotation :!class /Script/Engine.Pawn))))) AxisValue false)
  (if (Variables|Default|Getrunningshake)
    (Utilities|FlowControl|FlipFlop
      (:A
        (Game|Feedback|ClientStartCameraShake _returnvalue "/Game/Blueprints/CameraShakewhilerunning.CameraShakewhilerunning_C" 1.0 "CameraLocal" "0, 0, 0"))
      (:B
        (Game|Feedback|ClientStartCameraShake _returnvalue "/Game/Blueprints/CameraShakewhilerunning.CameraShakewhilerunning_C" 1.0 "CameraLocal" "0, 0, 0")))
    (else
      (Utilities|FlowControl|FlipFlop
        (:A
          (Game|Feedback|ClientStartCameraShake _returnvalue "/Game/Blueprints/CameraShakewhilewalking.CameraShakewhilewalking_C" (stale Input|AxisEvents|InputAxisLeft/Right AxisValue) "CameraLocal" "0, 0, 0"))
        (:B
          (Game|Feedback|ClientStartCameraShake _returnvalue "/Game/Blueprints/CameraShakewhilewalking.CameraShakewhilewalking_C" AxisValue "CameraLocal" "0, 0, 0"))))))

(event Input|AxisEvents|InputAxisLeft/Right
  (params (AxisValue :type Float%20%28single-precision%29))
  (bind _returnvalue (Game|GetPlayerController 0))
  (Pawn|Input|AddMovementInput (Math|Vector|GetRightVector (Math|Rotator|MakeRotator 0.0 0.0 (.Yaw (Math|Rotator|BreakRotator (Pawn|GetControlRotation :!class /Script/Engine.Pawn))))) AxisValue false)
  (if (Variables|Default|Getrunningshake)
    (Utilities|FlowControl|FlipFlop
      (:A
        (Game|Feedback|ClientStartCameraShake _returnvalue "/Game/Blueprints/CameraShakewhilerunning.CameraShakewhilerunning_C" 1.0 "CameraLocal" "0, 0, 0"))
      (:B
        (Game|Feedback|ClientStartCameraShake _returnvalue "/Game/Blueprints/CameraShakewhilerunning.CameraShakewhilerunning_C" 1.0 "CameraLocal" "0, 0, 0")))
    (else
      (Utilities|FlowControl|FlipFlop
        (:A
          (Game|Feedback|ClientStartCameraShake _returnvalue "/Game/Blueprints/CameraShakewhilewalking.CameraShakewhilewalking_C" AxisValue "CameraLocal" "0, 0, 0"))
        (:B
          (Game|Feedback|ClientStartCameraShake _returnvalue "/Game/Blueprints/CameraShakewhilewalking.CameraShakewhilewalking_C" (stale Input|AxisEvents|InputAxisForward/Backward AxisValue) "CameraLocal" "0, 0, 0"))))))

(event Input|AxisEvents|InputAxisLookUp/LookDown
  (params (AxisValue :type Float%20%28single-precision%29))
  (Pawn|Input|AddControllerPitchInput AxisValue))

(event Input|AxisEvents|InputAxisLookDown/LookUp
  (params (AxisValue :type Float%20%28single-precision%29))
  (Pawn|Input|AddControllerYawInput AxisValue))

(event Input|KeyboardEvents|F
  (params (Key :type Key%20Structure :default "None"))
  (:Pressed
    (if (Variables|Default|Getpickeduptorch)
      (Utilities|FlowControl|FlipFlop
        (:A
          (Rendering|SetVisibility (Variables|Default|GetSpotLight) true false))
        (:B
          (Rendering|SetVisibility (Variables|Default|GetSpotLight) false false))))))

(fn ConstructionScript)

(fn Startbrr
  (Variables|/Script/Engine.CharacterMovementComponent|SetMaxWalkSpeed (Variables|Character|GetCharacterMovement) (Variables|Default|GetSprint)))

(fn Stopbrr
  (Variables|/Script/Engine.CharacterMovementComponent|SetMaxWalkSpeed (Variables|Character|GetCharacterMovement) (Variables|Default|GetWalking)))