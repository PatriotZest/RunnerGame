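; Collectable pickup actor that the player collects by pressing Interact while standing inside its trigger box.
; Box overlaps with the FPSmovement player enable and disable the actor's input, so the key only works in range.
; On Interact it decrements the Collectables counter on FPSGamemode, adds a newly created Collectable_widget_bp to the viewport, then destroys itself.
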(event OnComponentBeginOverlap(Box)
  (params (OverlappedComponent :type Primitive%20Component%20Object%20Reference) (OtherActor :type Actor%20Object%20Reference) (OtherComp :type Primitive%20Component%20Object%20Reference) (OtherBodyIndex :type Integer) (bFromSweep :type Boolean) (SweepResult :type Hit%20Result%20Structure%20%28by%20ref%29))
  (Utilities|Casting|CastToFPSmovement OtherActor)
  (Input|EnableInput (Game|GetPlayerController 0)))

(event OnComponentEndOverlap(Box)
  (params (OverlappedComponent :type Primitive%20Component%20Object%20Reference) (OtherActor :type Actor%20Object%20Reference) (OtherComp :type Primitive%20Component%20Object%20Reference) (OtherBodyIndex :type Integer))
  (Utilities|Casting|CastToFPSmovement OtherActor)
  (Input|DisableInput (Game|GetPlayerController 0)))

(event EventBeginPlay)

(event Input|ActionEvents|InputActionInteract
  (params (Key :type Key%20Structure :default "None"))
  (:Pressed
    (bind _asfpsgamemode (Utilities|Casting|CastToFPSGamemode (Game|GetGameMode)))
    (bind _result (Math|Integer|DecrementInt (Variables|/Game/Blueprints/FPSGamemode.FPSGamemode_C|GetCollectables%20 _asfpsgamemode))
      (:%20%20
        (Variables|/Game/Blueprints/FPSGamemode.FPSGamemode_C|SetCollectables%20 _asfpsgamemode _result)
        (bind _returnvalue (UserInterface|CreateWidget "/Game/Level/Main_Menu_Widgets/Collectable_widget_bp.Collectable_widget_bp_C"))
        (UserInterface|Viewport|AddtoViewport _returnvalue 0)
        (Actor|DestroyActor)))))

(fn ConstructionScript)